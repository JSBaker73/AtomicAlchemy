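; A component that lets its owning actor be picked up and dropped, with special handling for electrons and atoms.
; Pickup and Drop check owner tags and forward grab or release messages to Electron and Atom actors, while other owners attach to the given component or detach, keeping world transforms.
; BeginPlay enables overlap events on static mesh actor owners.
; The electron attach, connect and detach functions are stubs returning false or zero.
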(event EventBeginPlay
  (bind _asstatic_mesh_actor (Utilities|Casting|CastToStaticMeshActor (Components|GetOwner)))
  (Variables|/Script/Engine.PrimitiveComponent|SetbGenerateOverlapEvents (Variables|/Script/Engine.StaticMeshActor|GetStaticMeshComponent _asstatic_mesh_actor) true))

(event EventPickup
  (params (AttachTo :type Scene%20Component%20Object%20Reference))
  (bind _returnvalue (Components|GetOwner))
  (if (Actor|ActorHasTag _returnvalue "Electron")
    (Class|ElectronInterface|GrabElectron(Message) _returnvalue AttachTo)
    (elif (Actor|ActorHasTag _returnvalue "Atom")
      (Class|NucleusInterface|GrabNucleus(Message) _returnvalue AttachTo)
      (else
        (Transformation|AttachComponentToComponent (VehicleSound|GetRootComponent _returnvalue) AttachTo "None" "KeepWorld" "KeepWorld" "KeepWorld" false)))))

(event EventDrop
  (bind _returnvalue (Components|GetOwner))
  (if (Actor|ActorHasTag _returnvalue "Electron")
    (Class|ElectronInterface|ReleaseElectron(Message) _returnvalue)
    (elif (Actor|ActorHasTag _returnvalue "Atom")
      (Class|NucleusInterface|ReleaseNucleus(Message) _returnvalue)
      (else
        (Transformation|DetachFromActor _returnvalue "KeepWorld" "KeepWorld" "KeepWorld")))))

(fn AttachElectron
  (params (Electron :type Actor%20Object%20Reference))
  (return false "0, 0, 0"))

(fn ConnectElectron
  (params (Electron :type Actor%20Object%20Reference))
  (return false))

(fn DetachElectron
  (params (Electron :type Actor%20Object%20Reference))
  (return false))
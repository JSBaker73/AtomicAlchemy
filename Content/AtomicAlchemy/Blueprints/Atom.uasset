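; Atom actor for a motion-controller chemistry game, deriving its valence shell from AtomicNumber and spawning orbiting Electrons.
; Hand overlap stops it, fixing electrons at paired angles and filling vacancies with EmptyElectron placeholders that highlight near other atoms or electrons.
; Grabbed nuclei follow the hand; on release, Tick eases them along the throw, then to the nearest free AnchorPoint.
; Connected atoms forward stop, start, grab and release to their Molecule.
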(event Collision|EventActorEndOverlap
  (params (OtherActor :type Actor%20Object%20Reference))
  (bind _molecule (Variables|Default|GetMolecule))
  (Utilities|Casting|CastToAtom OtherActor
    (:then
      _)
    (:CastFailed
      (Utilities|Casting|CastToElectron OtherActor
        (:then
          _)
        (:CastFailed
          (Utilities|Casting|CastToBP_MotionController OtherActor)))))
  (if (Variables|Default|GetConnected)
    (bind _clear (Default|CheckifAtomsAreStopped _molecule))
    (if _clear
      (Class|MoleculeInterface|StartMolecule(Message) _molecule))
    (else
      (bind _clear_2 (CallFunction|CheckifStillStopped))
      (if _clear_2
        (CallFunction|StartAtom)))))

(event EventBeginPlay
  (bind _atomicnumber (Variables|Default|GetAtomicNumber))
  ;[0 0 0] Begin Play
  (Variables|Default|SetElectronsNeeded _atomicnumber)
  (bind _array_element (Utilities|Array|ForEachLoopwithBreak (Variables|Default|GetAtomicShells) :!label _label)
    (:LoopBody
      (if (> (- (Variables|Default|GetElectronsNeeded) _array_element) 0)
        (Variables|Default|SetElectronsNeeded (- (Variables|Default|GetElectronsNeeded) _array_element))
        (else
          (Variables|Default|SetValenceCapacity _array_element)
          (goto _label Break))))
    (:Completed
      (Utilities|Array|Resize (Variables|Default|GetInnerElectrons) (- _atomicnumber (Variables|Default|GetElectronsNeeded)))
      (for _index (range 0 (- (- _atomicnumber (Variables|Default|GetElectronsNeeded)) 1))
        _)
      (Utilities|Array|Resize (Variables|Default|GetValenceElectrons) (Variables|Default|GetValenceCapacity))
      (for _index_2 (range 0 (- (Variables|Default|GetElectronsNeeded) 1))
        (CallFunction|GenerateValenceElectron))
      (Variables|Default|SetConstructed true))))

(event EventElectronReleased
  (bind _molecule (Variables|Default|GetMolecule))
  (if (Variables|Default|GetConnected)
    (bind _clear (Default|CheckifAtomsAreStopped _molecule))
    (if _clear
      (Class|MoleculeInterface|StartMolecule(Message) _molecule))
    (else
      (bind _clear_2 (CallFunction|CheckifStillStopped))
      (if _clear_2
        (CallFunction|StartAtom)))))

(event EventGrabNucleus
  (params (GrabbedBy :type Scene%20Component%20Object%20Reference))
  (if (Variables|Default|GetConnected)
    (Class|MoleculeInterface|GrabMolecule(Message) (Variables|Default|GetMolecule) GrabbedBy)
    (else
      (Variables|Default|SetCurrentState "NewEnumerator2")
      (Transformation|AttachComponentToComponent GrabbedBy "None" "KeepWorld" "KeepWorld" "KeepWorld" true)
      (Variables|Default|SetLerping false)
      (Variables|Default|SetThrown false))))

(event EventReleaseNucleus
  (if (Variables|Default|GetConnected)
    (Class|MoleculeInterface|ReleaseMolecule(Message) (Variables|Default|GetMolecule))
    (else
      (bind _clear (CallFunction|CheckifStillStopped))
      (if _clear
        (Variables|Default|SetCurrentState "NewEnumerator0")
        (else
          (Variables|Default|SetCurrentState "NewEnumerator1")))
      (Transformation|DetachFromActor "KeepWorld" "KeepWorld" "KeepWorld")
      (bind _found (CallFunction|FindAnchor))
      (if _found
        (Utilities|FlowControl|Sequence
          (:then_0
            (CallFunction|SetThrowPoint))
          (:then_1
            (Variables|Default|SetThrown true))
          (:then_2
            (Variables|Default|SetLerpTime 0.0))
          (:then_3
            (Variables|Default|SetLerping false)))))))

(event EventTick
  (params (DeltaSeconds :type Float%20%28single-precision%29))
  (bind _anchorpoint (Variables|Default|GetAnchorPoint))
  (bind _returnvalue (Transformation|GetActorLocation _anchorpoint))
  (switch Utilities|FlowControl|Switch|SwitchonNucleusStates (Variables|Default|GetCurrentState)
    (:NewEnumerator0
      (if (Variables|Default|GetLerping) :!label _label
        (if (!= 0 _anchorpoint)
          (bind (_complete _lerptime) (CallFunction|Lerp DeltaSeconds (Variables|Default|GetLerpSpeed)))
          (if _complete
            (Variables|Default|SetThrown false)
            (Variables|Default|SetLerping false)
            (Transformation|SetActorLocation _returnvalue false false)
            (else
              (Transformation|SetActorLocation (Math|Interpolation|Ease "EaseInOut" _lerptime (Transformation|GetActorLocation) _returnvalue 2.0) false false))))
        (elif (Variables|Default|GetThrown)
          (bind (_complete_2 _lerptime_2) (CallFunction|Lerp DeltaSeconds (Variables|Default|GetVelocity)))
          (if _complete_2
            (Transformation|SetActorLocation (Variables|Default|GetTargetPoint) false false)
            (Variables|Default|SetThrown false)
            (Variables|Default|SetLerping true)
            (else
              (Transformation|SetActorLocation (Math|Interpolation|Ease "EaseOut" _lerptime_2 (Variables|Default|GetThrowPoint) (Variables|Default|GetTargetPoint) 2.0) false false))))))
    (:NewEnumerator1
      (goto _label))
    (:NewEnumerator2
      (Variables|Default|SetThrowPoint (Variables|Default|GetTargetPoint))
      (Variables|Default|SetTargetPoint (Transformation|GetActorLocation))
      (Variables|Default|SetVelocity DeltaSeconds))))

(event Collision|EventActorBeginOverlap
  (params (OtherActor :type Actor%20Object%20Reference))
  (if (Variables|Default|GetConstructed) :!label _label
    (Utilities|Casting|CastToAtom OtherActor
      (:then
        (CallFunction|HighlightEmptyElectrons true :!label _label_2))
      (:CastFailed
        (bind _aselectron (Utilities|Casting|CastToElectron OtherActor)
          (:then
            (if (not (== (Variables|/Game/AtomicAlchemy/Blueprints/Electron.Electron_C|GetAtom1 _aselectron) self))
              (goto _label_2)))
          (:CastFailed
            (Utilities|Casting|CastToBP_MotionController OtherActor)
            (if (Utilities|Enum|NotEqual(Enum) (Variables|Default|GetCurrentState) "NewEnumerator1")
              (if (Variables|Default|GetConnected)
                (Class|MoleculeInterface|StopMolecule(Message) (Variables|Default|GetMolecule))
                (else
                  (CallFunction|StopAtom))))))))
    (else
      (Utilities|FlowControl|Delay 0.2)
      (goto _label))))

(event EventStartAtom
  (bind _valenceelectrons (Variables|Default|GetValenceElectrons))
  (Variables|Default|SetCurrentState "NewEnumerator0")
  (for (_array_element _array_index) _valenceelectrons
    (if (!= _array_element 0)
      (bind _aselectron (Utilities|Casting|CastToElectron _array_element)
        (:then
          (Class|ElectronInterface|StartElectron(Message) _aselectron))
        (:CastFailed
          (Actor|DestroyActor _array_element)
          (Utilities|Array|SetArrayElem _valenceelectrons _array_index 0))))))

(event EventStopAtom
  (bind _self self)
  (bind _valencecapacity (Variables|Default|GetValenceCapacity))
  (bind _valenceelectrons (Variables|Default|GetValenceElectrons))
  (Variables|Default|SetCurrentState "NewEnumerator1")
  (for (_array_element _array_index) _valenceelectrons
    (if (!= _array_element 0)
      (bind _stoprot (CallFunction|CreateStoppdPosition _array_index _valencecapacity))
      (Class|ElectronInterface|StopElectron(Message) _array_element _stoprot)
      (else
        (bind _stoprot_2 (CallFunction|CreateStoppdPosition _array_index _valencecapacity))
        (bind _returnvalue (Game|SpawnActorfromClass "/Game/AtomicAlchemy/Blueprints/EmptyElectron.EmptyElectron_C" (Math|Conversions|ToTransform(Vector) (Math|Vector|MakeVector 0.0 0.0 1.0)) "Undefined" 0 0))
        (Utilities|Array|SetArrayElem _valenceelectrons _array_index _returnvalue)
        (Utilities|FlowControl|Sequence
          (:then_0
            (Variables|/Game/AtomicAlchemy/Blueprints/EmptyElectron.EmptyElectron_C|SetFilled _returnvalue (Utilities|Array|ContainsItem (Variables|Default|GetConnections) _array_index)))
          (:then_1
            (Variables|/Game/AtomicAlchemy/Blueprints/EmptyElectron.EmptyElectron_C|SetStopRot _returnvalue _stoprot_2))
          (:then_2
            (Variables|/Game/AtomicAlchemy/Blueprints/EmptyElectron.EmptyElectron_C|SetAtom1 _returnvalue _self))
          (:then_3
            (Transformation|AttachActorToActor _returnvalue _self "None" "KeepRelative" "KeepRelative" "KeepRelative" true)))))))

(fn ConstructionScript)

(fn CreateSingleOrbitDirection
  (params (OrbitNumber :type Integer) (MaxOrbits :type Integer))
  (bind _returnvalue (Math|Conversions|ToFloat(Integer) OrbitNumber))
  (bind _returnvalue_2 (Math|Conversions|ToFloat(Integer) MaxOrbits))
  (bind _returnvalue_3 (/ _returnvalue _returnvalue_2))
  (bind _returnvalue_4 (* _returnvalue_3 1.8e+02))
  (return (Math|Trig|Sin(Degrees) _returnvalue_4) (Math|Trig|Cos(Degrees) _returnvalue_4)))

(fn CheckHandOverlap)

(fn CreateStoppdPosition
  (params (OrbitNumber :type Integer) (MaxOrbits :type Integer))
  (return (+ (* (/ (Math|Conversions|ToFloat(Integer) (/ OrbitNumber 2)) (Math|Conversions|ToFloat(Integer) (/ MaxOrbits 2))) 3.6e+02) (* (Math|Conversions|ToFloat(Integer) (- (* (Math|Integer|%(Integer) OrbitNumber 2) 2) 1)) 15.0))))

(fn CheckifStillStopped
  (bind _self self)
  (bind _array_element (Utilities|Array|ForEachLoopwithBreak (Collision|GetOverlappingActors (Variables|Default|GetSphere) 0 :!class /Script/Engine.PrimitiveComponent))
    (:LoopBody
      (bind _asatom (Utilities|Casting|CastToAtom _array_element)
        (:then
          (if (!= _self _asatom)
            (LocalVariables|SetObjectClear false :!label _label)))
        (:CastFailed
          (bind _aselectron (Utilities|Casting|CastToElectron _array_element)
            (:then
              (if (and (!= _self (Variables|/Game/AtomicAlchemy/Blueprints/Electron.Electron_C|GetAtom1 _aselectron)) (!= _self (Variables|/Game/AtomicAlchemy/Blueprints/Electron.Electron_C|GetAtom2 _aselectron)))
                (goto _label)))
            (:CastFailed
              (Utilities|Casting|CastToBP_MotionController _array_element)
              (LocalVariables|SetHandClear false))))))
    (:Completed
      (if (LocalVariables|GetObjectClear)
        (CallFunction|HighlightEmptyElectrons false))
      (if (Math|Boolean|NANDBoolean (LocalVariables|GetObjectClear) (LocalVariables|GetHandClear))
        (return false)
        (else
          (bind _array_element_2 (Utilities|Array|ForEachLoopwithBreak (Variables|Default|GetValenceElectrons))
            (:LoopBody
              (bind _aselectron_2 (Utilities|Casting|CastToElectron _array_element_2))
              (if (Utilities|Enum|Equal(Enum) (Variables|/Game/AtomicAlchemy/Blueprints/Electron.Electron_C|GetCurrentState _aselectron_2) "NewEnumerator4")
                (return false)))
            (:Completed
              (return true))))))))

(fn GenerateValenceElectron
  (bind _valenceelectrons (Variables|Default|GetValenceElectrons))
  (bind _valencecapacity (Variables|Default|GetValenceCapacity))
  (bind _returnvalue (Game|SpawnActorfromClass "/Game/AtomicAlchemy/Blueprints/Electron.Electron_C" (Transformation|GetActorTransform) "Undefined" 0 0))
  (if (Utilities|Array|ContainsItem _valenceelectrons _returnvalue)
    (bind (_orbitdirectionx _orbitdirectiony) (CallFunction|CreateSingleOrbitDirection (Utilities|Array|FindItem _valenceelectrons _returnvalue) _valencecapacity))
    (Default|CreateSingleOrbit _returnvalue (Math|Vector|MakeVector _orbitdirectionx 0.0 _orbitdirectiony))
    (Variables|/Game/AtomicAlchemy/Blueprints/Electron.Electron_C|SetAtom1 _returnvalue self :!label _label)
    (Class|ElectronInterface|ReleaseElectron(Message) _returnvalue)
    (return)
    (else
      (bind _index (Utilities|FlowControl|ForLoopwithBreak 0 (- _valencecapacity 1))
        (:LoopBody
          (if (== (Utilities|Array|Get(acopy) _valenceelectrons (|ValenceOffset_2 _index _index _valencecapacity)) 0)
            (Utilities|Array|SetArrayElem _valenceelectrons (|ValenceOffset_2 _index _index _valencecapacity) _returnvalue)
            (bind (_orbitdirectionx_2 _orbitdirectiony_2) (CallFunction|CreateSingleOrbitDirection (|ValenceOffset_2 _index _index _valencecapacity) _valencecapacity))
            (Default|CreateSingleOrbit _returnvalue (Math|Vector|MakeVector _orbitdirectionx_2 0.0 _orbitdirectiony_2))
            (goto _label)))))))

(fn HighlightEmptyElectrons
  (params (On :type Boolean))
  (for _array_element (Variables|Default|GetValenceElectrons)
    (bind _asempty_electron (Utilities|Casting|CastToEmptyElectron _array_element))
    (if (Variables|/Game/AtomicAlchemy/Blueprints/EmptyElectron.EmptyElectron_C|GetFilled _asempty_electron)
      (if On
        (Rendering|Material|SetVectorParameterValue (Variables|/Game/AtomicAlchemy/Blueprints/EmptyElectron.EmptyElectron_C|GetMaterial _asempty_electron) "BaseColor" "(R=0.000000,G=0.000000,B=0.000000,A=1.000000)" :!class /Script/Engine.MaterialInstanceDynamic)
        (else
          (Rendering|Material|SetVectorParameterValue (Variables|/Game/AtomicAlchemy/Blueprints/EmptyElectron.EmptyElectron_C|GetMaterial _asempty_electron) "BaseColor" "(R=0.050000,G=0.050000,B=0.050000,A=1.000000)" :!class /Script/Engine.MaterialInstanceDynamic :!label _label)))
      (elif On
        (Rendering|Material|SetVectorParameterValue (Variables|/Game/AtomicAlchemy/Blueprints/EmptyElectron.EmptyElectron_C|GetMaterial _asempty_electron) "BaseColor" "(R=0.250000,G=0.500000,B=0.250000,A=1.000000)" :!class /Script/Engine.MaterialInstanceDynamic)
        (else
          (goto _label))))))

(fn Lerp
  (params (DeltaTime :type Float%20%28single-precision%29) (LerpSpeed :type Float%20%28single-precision%29))
  (if (>= (+ (Variables|Default|GetLerpTime) (* DeltaTime LerpSpeed)) 1.0)
    (Variables|Default|SetLerpTime 0.0)
    (return true 0.0)
    (else
      (bind _output_get (Variables|Default|SetLerpTime (+ (Variables|Default|GetLerpTime) (* DeltaTime LerpSpeed))))
      (return false _output_get))))

(fn SetThrowPoint
  (bind _throwpoint (Variables|Default|GetThrowPoint))
  (Variables|Default|SetTargetPoint (/ (- (Variables|Default|GetTargetPoint) _throwpoint) (Variables|Default|GetVelocity)))
  (bind _output_get (Variables|Default|SetVelocity (Math|Vector|VectorLength (Variables|Default|GetTargetPoint))))
  (Variables|Default|SetTargetPoint (+ _throwpoint (* (Variables|Default|GetTargetPoint) 1.0)))
  (Variables|Default|SetVelocity (Math|Float|Power (/ _output_get 1e+02) -0.1)))

(fn FindAnchor
  (if (== (Variables|Default|GetAnchorPoint) 0)
    _
    (else
      (bind _asanchor_point (Utilities|Casting|CastToAnchorPoint (Variables|Default|GetAnchorPoint)))
      (Variables|/Game/AtomicAlchemy/Blueprints/AnchorPoint.AnchorPoint_C|SetObject _asanchor_point 0)))
  (bind _outactors (Actor|GetAllActorswithTag "Anchor"))
  (bind _array_element (Utilities|Array|ForEachLoopwithBreak _outactors)
    (:LoopBody
      (bind _asanchor_point_2 (Utilities|Casting|CastToAnchorPoint _array_element))
      (if (== (Variables|/Game/AtomicAlchemy/Blueprints/AnchorPoint.AnchorPoint_C|GetObject _asanchor_point_2) 0)
        (if (== (Variables|Default|GetAnchorPoint) 0)
          (Variables|Default|SetAnchorPoint _asanchor_point_2 :!label _label)
          (elif (< (Transformation|GetDistanceTo _asanchor_point_2) (Transformation|GetDistanceTo (Variables|Default|GetAnchorPoint)))
            (goto _label)))))
    (:Completed
      (if (== (Variables|Default|GetAnchorPoint) 0)
        (return false)
        (else
          (bind _asanchor_point_3 (Utilities|Casting|CastToAnchorPoint (Variables|Default|GetAnchorPoint)))
          (Variables|/Game/AtomicAlchemy/Blueprints/AnchorPoint.AnchorPoint_C|SetObject _asanchor_point_3 self)
          (return true))))))

(fn AttachElectron
  (params (Electron :type Actor%20Object%20Reference))
  (bind _returnvalue (Utilities|Array|AddUnique (Variables|Default|GetValenceElectrons) Electron))
  (if (== _returnvalue -1)
    (return false "0, 0, 0")
    (else
      (bind (_array_element _array_index) (Utilities|Array|ForEachLoopwithBreak (Variables|Default|GetValenceElectrons))
        (:LoopBody
          (if (or (== "/Game/AtomicAlchemy/Blueprints/EmptyElectron.EmptyElectron_C" (Utilities|GetClass _array_element)) (== 0 _array_element))
            (Actor|DestroyActor _array_element)
            (Utilities|Array|SetArrayElem (Variables|Default|GetValenceElectrons) _array_index Electron)
            (bind _returnvalue_2 (Utilities|Array|AddUnique (Variables|Default|GetConnections) _array_index))
            (if (not (== _returnvalue_2 -1))
              (bind (_orbitdirectionx _orbitdirectiony) (CallFunction|CreateSingleOrbitDirection _array_index (Variables|Default|GetValenceCapacity)))
              (return true (Math|Vector|MakeVector _orbitdirectionx _orbitdirectiony 0.0)))))
        (:Completed
          (return false "0, 0, 0"))))))

(fn ConnectElectron
  (params (Electron :type Actor%20Object%20Reference))
  (return false))

(fn DetachElectron
  (params (Electron :type Actor%20Object%20Reference))
  (bind _valenceelectrons (Variables|Default|GetValenceElectrons))
  (if (Utilities|Array|ContainsItem _valenceelectrons Electron)
    (Utilities|Array|SetArrayElem _valenceelectrons (Utilities|Array|FindItem _valenceelectrons Electron) 0)
    (return true)
    (else
      (return false))))
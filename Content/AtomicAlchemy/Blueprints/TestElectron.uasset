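; Grabbable electron actor for an atom-building game that can be loose, held, stopped, or bound to one or two atoms.
; On BeginPlay it registers with its atom via an attach message; in single orbit, Tick circles that atom, easing back after release.
; While held, it detects overlapping "Atom"-tagged actors and stretches a spline mesh to the first atom.
; Release sets the state from those connections; double orbit has no movement, and its own attach/connect/detach functions are stubs.
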(event EventBeginPlay
  (bind _returnvalue (Actor|GetAttachParentActor))
  (bind _self self)
  (bind _returnvalue_2 (== 0 _returnvalue))
  (Rendering|SetVisibility (Variables|Default|GetSplineMesh) false false)
  (if (== 0 (Variables|Default|GetAtom2))
    (if (== 0 (Variables|Default|GetAtom1))
      (if _returnvalue_2
        (Variables|Default|SetCurrentState "NewEnumerator5" :!label _label)
        (else
          (Variables|Default|SetAtom1 _returnvalue)
          (Variables|Default|SetCurrentState "NewEnumerator0" :!label _label_2)
          (bind (_complete _orbitdirection) (Class|ElectronInterface|AttachElectron(Message) (stale _output_get) _self))
          (if _complete
            (CallFunction|CreateSingleOrbit _orbitdirection)
            (else
              (goto _label)))))
      (else
        (Transformation|AttachActorToActor _returnvalue "None" "KeepRelative" "KeepRelative" "KeepRelative" true)
        (goto _label_2)))
    (else
      (if (== 0 (Variables|Default|GetAtom1))
        (if _returnvalue_2
          (Variables|Default|SetAtom2 0)
          (goto _label)
          (else
            (bind _output_get (Variables|Default|SetAtom1 _returnvalue))))
        (else
          (Transformation|AttachActorToActor _returnvalue "None" "KeepRelative" "KeepRelative" "KeepRelative" true)))
      (Variables|Default|SetCurrentState "NewEnumerator6")
      (bind _complete_2 (Class|ElectronInterface|AttachElectron(Message) _output_get _self))
      (if _complete_2
        (bind _complete_3 (CallFunction|ConnectElectron _self))
        (if _complete_3
          _)
        (else
          (goto _label))))))

(event EventTick
  (params (DeltaSeconds :type Float%20%28single-precision%29))
  (bind _atom1 (Variables|Default|GetAtom1))
  (switch Utilities|FlowControl|Switch|SwitchonElectronStates (Variables|Default|GetCurrentState)
    (:NewEnumerator0
      (if (>= (+ (Variables|Default|GetAngle) (* DeltaSeconds (Variables|Default|GetRotSpeed))) 3.6e+02)
        (Variables|Default|SetAngle (+ (Variables|Default|GetAngle) (* DeltaSeconds (Variables|Default|GetRotSpeed))))
        (else
          (Variables|Default|SetAngle (- (+ (Variables|Default|GetAngle) (* DeltaSeconds (Variables|Default|GetRotSpeed))) 3.6e+02))))
      (bind _outpoint (CallFunction|GetRotationAroundPoint (Transformation|GetActorLocation _atom1) (Math|Vector|RotateVectorAroundAxis (Variables|Default|GetOrbit1) (Variables|Default|GetAngle) (Variables|Default|GetAxis)) (Variables|Default|GetDistance)))
      (if (Variables|Default|GetLerping)
        (if (>= (+ (Variables|Default|GetLerpTime) (* DeltaSeconds (Variables|Default|GetLerpSpeed))) 1.0)
          (Transformation|SetActorLocation _outpoint false false :!label _label)
          (else
            (bind _output_get (Variables|Default|SetLerpTime (+ (Variables|Default|GetLerpTime) (* DeltaSeconds (Variables|Default|GetLerpSpeed)))))
            (Transformation|SetActorLocation (Math|Interpolation|Ease "EaseInOut" _output_get (Transformation|GetActorLocation) _outpoint 2.0) false false)))
        (else
          (goto _label))))
    (:NewEnumerator4
      (CallFunction|UpdateOverlapConnection)
      (if (not (== _atom1 0))
        (CallFunction|UpdateSplineandMesh)))))

(event EventGrabElectron
  (params (GrabbedBy :type Scene%20Component%20Object%20Reference))
  (Components|Activation|Deactivate (Variables|Default|GetElectronTrail))
  (Physics|SetSimulatePhysics (Variables|Debug|GetStaticMeshComponent) false)
  (if (Utilities|Enum|Equal(Enum) (Variables|Default|GetCurrentState) "NewEnumerator5")
    _
    (else
      (Transformation|DetachFromActor "KeepWorld" "KeepWorld" "KeepWorld")))
  (Variables|Default|SetCurrentState "NewEnumerator4")
  (Transformation|AttachComponentToComponent GrabbedBy "None" "KeepWorld" "KeepWorld" "KeepWorld" true)
  (if (not (== (Variables|Default|GetAtom1) 0))
    (Rendering|SetVisibility (Variables|Default|GetSplineMesh) true false)))

(event EventReleaseElectron
  (CallFunction|UpdateConnectionState)
  (Variables|Default|SetLerping true)
  (Transformation|DetachFromActor "KeepWorld" "KeepWorld" "KeepWorld")
  (switch Utilities|FlowControl|Switch|SwitchonElectronStates (Variables|Default|GetCurrentState)
    (:NewEnumerator0
      (Rendering|SetVisibility (Variables|Default|GetSplineMesh) false false :!label _label))
    (:NewEnumerator6
      (goto _label))
    (:NewEnumerator3
      _))
  (Components|Activation|Activate (Variables|Default|GetElectronTrail) false)
  (Transformation|AttachActorToActor (Variables|Default|GetAtom1) "None" "KeepWorld" "KeepWorld" "KeepWorld" true))

(fn ConstructionScript)

(fn GetRotationAroundPoint
  (params (Center :type Vector) (Rotation :type Vector) (Distance :type Float%20%28single-precision%29))
  (return (+ Center (* Rotation Distance))))

(fn UpdateConnectionState
  (bind _atom1 (Variables|Default|GetAtom1))
  (bind _atom2 (Variables|Default|GetAtom2))
  (if (== 0 _atom1)
    (Variables|Default|SetCurrentState "NewEnumerator5")
    (elif (== 0 _atom2)
      (Variables|Default|SetCurrentState "NewEnumerator0")
      (bind _astest_atom (Utilities|Casting|CastToTestAtom _atom1))
      (switch Utilities|FlowControl|Switch|SwitchonNucleusStates (Variables|/Game/AtomicAlchemy/Blueprints/TestAtom.TestAtom_C|GetCurrentState _astest_atom)
        (:NewEnumerator0
          _)
        (:NewEnumerator1
          (Variables|Default|SetCurrentState "NewEnumerator3" :!label _label))
        (:NewEnumerator2
          (goto _label)))
      (else
        (Variables|Default|SetCurrentState "NewEnumerator6")
        (bind _astest_atom_2 (Utilities|Casting|CastToTestAtom _atom2))
        (switch Utilities|FlowControl|Switch|SwitchonNucleusStates (Variables|/Game/AtomicAlchemy/Blueprints/TestAtom.TestAtom_C|GetCurrentState _astest_atom_2)
          (:NewEnumerator0
            _)
          (:NewEnumerator1
            (goto _label))
          (:NewEnumerator2
            (goto _label))))))
  (return))

(fn CreateSingleOrbit
  (params (Orbit1 :type Vector))
  (bind _output_get (Variables|Default|SetOrbit1 Orbit1))
  (Variables|Default|SetRotSpeed (+ (Variables|Default|GetRotSpeed) (Math|Random|RandomFloatinRange -2e+01 2e+01)))
  (Variables|Default|SetAngle (Math|Random|RandomFloatinRange 0.0 3.6e+02))
  (Variables|Default|SetAxis (Math|Vector|Normalize (Math|Vector|CrossProduct _output_get "0,1.000000, 0"))))

(fn UpdateSplineandMesh
  (bind _spline (Variables|Default|GetSpline))
  (bind (_location _tangent) (Spline|GetLocationandTangentatSplinePoint _spline 1 "Local"))
  (bind (_location_2 _tangent_2) (Spline|GetLocationandTangentatSplinePoint _spline 0 "Local"))
  (bind _output_get (LocalVariables|SetPoints (Utilities|Array|MakeArray (Transformation|GetWorldLocation (Variables|Default|GetElectron)) (Transformation|GetActorLocation (Variables|Default|GetAtom1)))))
  (Spline|SetSplinePoints _spline _output_get "World" true)
  (SplineMesh|SetStartandEnd (Variables|Default|GetSplineMesh) _location_2 _tangent_2 _location _tangent true :!class /Script/Engine.SplineMeshComponent) ; Set the tangents and position to build slightly bend the cylinder. All cylinders combined create a smooth arc.
)

(fn UpdateOverlapConnection
  (bind _array_element (Utilities|Array|ForEachLoopwithBreak (Collision|GetOverlappingActors (Variables|Debug|GetStaticMeshComponent) "/Script/Engine.Actor" :!class /Script/Engine.PrimitiveComponent))
    (:LoopBody
      (if (== 0 (Variables|Default|GetAtom1))
        (if (Actor|ActorHasTag _array_element "Atom")
          (Variables|Default|SetAtom1 _array_element)
          (return))
        (elif (not (== _array_element (Variables|Default|GetAtom1)))
          (if (Actor|ActorHasTag _array_element "Atom")
            (Variables|Default|SetAtom2 _array_element)
            (return)))))))

(fn AttachElectron
  (params (Electron :type Actor%20Object%20Reference))
  (return false "0, 0, 0"))

(fn ConnectElectron
  (params (Electron :type Actor%20Object%20Reference))
  (return false))

(fn DetachElectron
  (params (Electron :type Actor%20Object%20Reference))
  (return false))
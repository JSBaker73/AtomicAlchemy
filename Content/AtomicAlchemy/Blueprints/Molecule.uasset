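; Molecule actor in an atom-building VR game that groups atoms and connections so motion controllers can stop, grab and release it as one object.
; A controller overlap stops every atom; grabbing attaches the molecule to the grabber, and releasing detaches it.
; On overlap end or release, it restarts all atoms only if each passes its still-stopped check and no controller overlaps a connection.
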(event EventReleaseMolecule
  (bind _clear (CallFunction|CheckifAtomsAreStopped))
  (if _clear
    (CallFunction|StartMolecule))
  (Transformation|DetachFromActor "KeepWorld" "KeepWorld" "KeepWorld"))

(event EventGrabMolecule
  (params (GrabbedBy :type Scene%20Component%20Object%20Reference))
  (Variables|Default|SetCurrentState "NewEnumerator2")
  (Transformation|AttachComponentToComponent GrabbedBy "None" "KeepWorld" "KeepWorld" "KeepWorld" true))

(event EventStopMolecule
  (Variables|Default|SetCurrentState "NewEnumerator1")
  (for _array_element (Variables|Default|GetAtoms)
    (Class|NucleusInterface|StopAtom(Message) _array_element)))

(event EventStartMolecule
  (Variables|Default|SetCurrentState "NewEnumerator0")
  (for _array_element (Variables|Default|GetAtoms)
    (Class|NucleusInterface|StartAtom(Message) _array_element)))

(event Collision|EventActorBeginOverlap
  (params (OtherActor :type Actor%20Object%20Reference))
  (Utilities|Casting|CastToBP_MotionController OtherActor)
  (if (Utilities|Enum|NotEqual(Enum) (Variables|Default|GetCurrentState) "NewEnumerator1")
    (CallFunction|StopMolecule)))

(event Collision|EventActorEndOverlap
  (params (OtherActor :type Actor%20Object%20Reference))
  (Utilities|Casting|CastToBP_MotionController OtherActor)
  (bind _clear (CallFunction|CheckifAtomsAreStopped))
  (if _clear
    (CallFunction|StartMolecule)))

(fn ConstructionScript)

(fn CheckifAtomsAreStopped
  (for _array_element (Variables|Default|GetAtoms)
    (bind _clear (Default|CheckifStillStopped _array_element))
    (if (not _clear)
      (return false)))
  (for _array_element_2 (Variables|Default|GetConnections)
    (for _array_element_3 (Collision|GetOverlappingActors _array_element_2 "/Game/VirtualRealityBP/Blueprints/BP_MotionController.BP_MotionController_C" :!class /Script/Engine.Actor)
      (return false)))
  (return true))
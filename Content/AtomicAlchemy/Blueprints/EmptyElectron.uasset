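; Empty electron slot on an atom that marks where an electron from another atom can go.
; On Tick, depending on atom state, it sits on a vertical ring that turns to face the VR headset, placed by StopRot and Distance around the atom's center.
; A Lerp timer eases it into that position while Lerping is set.
; Overlap with a foreign electron tints its dynamic material when unfilled; leaving restores a filled or empty color.
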(event EventTick
  (params (DeltaSeconds :type Float%20%28single-precision%29))
  (bind _returnvalue (Game|GetPlayerCameraManager 0))
  (bind (_devicerotation _deviceposition) (Class|HeadMountedDisplayFunctionLibrary|GetOrientationandPosition))
  (bind _atom1 (Variables|Default|GetAtom1))
  (bind _returnvalue_2 (Math|Vector|UnrotateVector _deviceposition _devicerotation))
  (bind _returnvalue_3 (Transformation|GetActorTransform _returnvalue))
  (bind _returnvalue_4 (Transformation|GetActorLocation _atom1))
  (bind _returnvalue_5 (Math|Transform|TransformLocation _returnvalue_3 _returnvalue_2))
  ;[0 0 0] Stopped
  (if (or (Utilities|Enum|NotEqual(Enum) (Variables|/Game/AtomicAlchemy/Blueprints/Atom.Atom_C|GetCurrentState _atom1) "NewEnumerator2") (Variables|Default|GetLerping))
    (bind _outpoint (CallFunction|GetRotationAroundPoint (Variables|Default|GetDistance) (Math|Vector|RotateVectorAroundAxis "0, 0,1.000000" (Variables|Default|GetStopRot) (Math|Vector|Normalize (- (Math|Vector|MakeVector (.x _returnvalue_4) (.y _returnvalue_4) 0.0) (Math|Vector|MakeVector (.x _returnvalue_5) (.y _returnvalue_5) 0.0)))) (Transformation|GetActorLocation _atom1)))
    (if (Variables|Default|GetLerping)
      (bind (_complete _lerptime) (CallFunction|Lerp DeltaSeconds))
      (if _complete
        (Variables|Default|SetLerping false)
        (Transformation|SetActorLocation _outpoint false false :!label _label)
        (else
          (Transformation|SetActorLocation (Math|Interpolation|Ease "EaseInOut" _lerptime (Transformation|GetActorLocation) _outpoint 2.0) false false)))
      (else
        (goto _label)))))

(event Collision|EventActorBeginOverlap
  (params (OtherActor :type Actor%20Object%20Reference))
  (if (not (Variables|Default|GetFilled))
    (bind _aselectron (Utilities|Casting|CastToElectron OtherActor))
    (if (!= (Variables|/Game/AtomicAlchemy/Blueprints/Electron.Electron_C|GetAtom1 _aselectron) (Variables|Default|GetAtom1))
      (Rendering|Material|SetVectorParameterValue (Variables|Default|GetMaterial) "BaseColor" "(R=0.100000,G=0.500000,B=0.100000,A=1.000000)" :!class /Script/Engine.MaterialInstanceDynamic))))

(event Collision|EventActorEndOverlap
  (params (OtherActor :type Actor%20Object%20Reference))
  (bind _material (Variables|Default|GetMaterial))
  (bind _aselectron (Utilities|Casting|CastToElectron OtherActor))
  (if (!= (Variables|/Game/AtomicAlchemy/Blueprints/Electron.Electron_C|GetAtom1 _aselectron) (Variables|Default|GetAtom1))
    (if (Variables|Default|GetFilled)
      (Rendering|Material|SetVectorParameterValue _material "BaseColor" "(R=0.000000,G=0.000000,B=0.000000,A=1.000000)" :!class /Script/Engine.MaterialInstanceDynamic)
      (else
        (Rendering|Material|SetVectorParameterValue _material "BaseColor" "(R=0.250000,G=0.500000,B=0.250000,A=1.000000)" :!class /Script/Engine.MaterialInstanceDynamic)))))

(fn ConstructionScript
  (bind _returnvalue (Rendering|Material|CreateDynamicMaterialInstance (Variables|Default|GetSphere) 0 0 :!class /Script/Engine.PrimitiveComponent))
  (Variables|Default|SetMaterial _returnvalue))

(fn Lerp
  (params (DeltaTime :type Float%20%28single-precision%29))
  (if (>= (+ (Variables|Default|GetLerpTime) (* DeltaTime (Variables|Default|GetLerpSpeed))) 1.0)
    (bind _output_get (Variables|Default|SetLerpTime 0.0))
    (return true _output_get)
    (else
      (bind _output_get_2 (Variables|Default|SetLerpTime (+ (Variables|Default|GetLerpTime) (* DeltaTime (Variables|Default|GetLerpSpeed)))))
      (return false _output_get_2))))

(fn GetRotationAroundPoint
  (params (Distance :type Float%20%28single-precision%29) (Rotation :type Vector) (Center :type Vector))
  (return (+ (* Rotation Distance) Center)))
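; Test atom Blueprint whose nucleus can be grabbed and released, and which manages electrons in a fixed number of valence slots.
; Grab and release attach or detach the atom, or its parent actor when connected, and update its state.
; AttachElectron fills even slots before odd via ValenceOffset, returning orbit directions spread over a half-circle in XZ; DetachElectron clears slots.
; ConnectElectron and CheckHandOverlap are stubs.
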(event EventBeginPlay
  (Utilities|Array|Resize (Variables|Default|GetValenceElectrons) (Variables|Default|GetValenceCapacity)))

(event EventTick
  (params (DeltaSeconds :type Float%20%28single-precision%29)))

(event EventGrabNucleus
  (params (GrabbedBy :type Scene%20Component%20Object%20Reference))
  (Variables|Default|SetCurrentState "NewEnumerator2")
  (Physics|SetSimulatePhysics (Variables|Debug|GetStaticMeshComponent) true)
  (if (Variables|Default|GetConnected)
    (Transformation|AttachComponentToComponent (Actor|GetParentActor) GrabbedBy "None" "KeepWorld" "KeepWorld" "KeepWorld" true)
    (else
      (Transformation|AttachComponentToComponent GrabbedBy "None" "KeepWorld" "KeepWorld" "KeepWorld" true))))

(event EventReleaseNucleus
  (Variables|Default|SetCurrentState "NewEnumerator0")
  (Physics|SetSimulatePhysics (Variables|Debug|GetStaticMeshComponent) true)
  (if (Variables|Default|GetConnected)
    (Transformation|DetachFromActor (Actor|GetParentActor) "KeepWorld" "KeepWorld" "KeepWorld")
    (else
      (Transformation|DetachFromActor "KeepWorld" "KeepWorld" "KeepWorld"))))

(fn ConstructionScript)

(fn CreateSingleOrbitDirection
  (params (OrbitNumber :type Integer) (MaxOrbits :type Integer))
  (bind _returnvalue (Math|Conversions|ToFloat(Integer) OrbitNumber))
  (bind _returnvalue_2 (Math|Conversions|ToFloat(Integer) MaxOrbits))
  (bind _returnvalue_3 (/ _returnvalue _returnvalue_2))
  (bind _returnvalue_4 (* _returnvalue_3 1.8e+02))
  (return (Math|Trig|Sin(Degrees) _returnvalue_4) (Math|Trig|Cos(Degrees) _returnvalue_4)))

(fn CheckHandOverlap)

(fn AttachElectron
  (params (Electron :type Actor%20Object%20Reference))
  (bind _valenceelectrons (Variables|Default|GetValenceElectrons))
  (bind _valencecapacity (Variables|Default|GetValenceCapacity))
  (if (Utilities|Array|ContainsItem _valenceelectrons Electron)
    (bind (_orbitdirectionx _orbitdriectionz) (CallFunction|CreateSingleOrbitDirection (Utilities|Array|FindItem _valenceelectrons Electron) _valencecapacity))
    (return true (Math|Vector|MakeVector _orbitdirectionx 0.0 _orbitdriectionz))
    (else
      (bind _index (Utilities|FlowControl|ForLoopwithBreak 0 (- _valencecapacity 1))
        (:LoopBody
          (if (== (Utilities|Array|Get(acopy) _valenceelectrons (|ValenceOffset _index _index _valencecapacity)) 0)
            (Utilities|Array|SetArrayElem _valenceelectrons (|ValenceOffset _index _index _valencecapacity) Electron)
            (bind (_orbitdirectionx_2 _orbitdriectionz_2) (CallFunction|CreateSingleOrbitDirection (|ValenceOffset _index _index _valencecapacity) _valencecapacity))
            (return true (Math|Vector|MakeVector _orbitdirectionx_2 0.0 _orbitdriectionz_2))))
        (:Completed
          (return false "0, 0, 0"))))))

(fn ConnectElectron
  (params (Electron :type Actor%20Object%20Reference))
  (return false))

(fn DetachElectron
  (params (Electron :type Actor%20Object%20Reference))
  (bind _valenceelectrons (Variables|Default|GetValenceElectrons))
  (if (Utilities|Array|ContainsItem _valenceelectrons Electron)
    (Utilities|Array|SetArrayElem _valenceelectrons (Utilities|Array|FindItem _valenceelectrons Electron) 0)
    (return true)
    (else
      (return false))))
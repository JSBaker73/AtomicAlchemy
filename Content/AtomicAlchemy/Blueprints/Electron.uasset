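; Electron actor for a VR atom game that orbits an Atom and can be grabbed, thrown and released.
; A Tick state machine rotates it in orbit or, when stopped, places it around the atom in a plane facing the headset.
; While held, it tracks overlapping atoms and stretches a spline-mesh connection.
; On release, hand motion sets an eased throw before it lerps back into place; double orbit is only stubbed.
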(event EventBeginPlay
  ;[0 0 0] BeginPlay
)

(event EventReleaseElectron
  (bind _splinemesh (Variables|Default|GetSplineMesh))
  ;[0 0 0] Grab and Release Electron
  (CallFunction|UpdateConnectionState)
  (Transformation|DetachFromActor "KeepWorld" "KeepWorld" "KeepWorld")
  (switch Utilities|FlowControl|Switch|SwitchonElectronStates (Variables|Default|GetCurrentState)
    (:NewEnumerator0
      (Components|Activation|Activate (Variables|Default|GetElectronTrail) false :!label _label))
    (:NewEnumerator6
      (CallFunction|CreateDoubleOrbit "0, 0, 0")
      (goto _label))
    (:NewEnumerator3
      _))
  (Transformation|AttachActorToActor (Variables|Default|GetAtom1) "None" "KeepWorld" "KeepWorld" "KeepWorld" true)
  (if (!= _splinemesh 0)
    (Actor|DestroyActor _splinemesh)
    (Utilities|FlowControl|Sequence
      (:then_0
        (CallFunction|SetThrowPoint))
      (:then_1
        (Variables|Default|SetThrown true))
      (:then_2
        (Variables|Default|SetLerpTime 0.0))
      (:then_3
        (Variables|Default|SetLerping false)))))

(event EventTick
  (params (DeltaSeconds :type Float%20%28single-precision%29))
  (bind _returnvalue (Game|GetPlayerCameraManager 0))
  (bind (_devicerotation _deviceposition) (Class|HeadMountedDisplayFunctionLibrary|GetOrientationandPosition))
  (bind _atom1 (Variables|Default|GetAtom1))
  (bind _returnvalue_2 (Math|Vector|UnrotateVector _deviceposition _devicerotation))
  (bind _returnvalue_3 (Transformation|GetActorTransform _returnvalue))
  (bind _returnvalue_4 (Transformation|GetActorLocation _atom1))
  (bind _returnvalue_5 (Math|Transform|TransformLocation _returnvalue_3 _returnvalue_2))
  (switch Utilities|FlowControl|Switch|SwitchonElectronStates (Variables|Default|GetCurrentState)
    (:NewEnumerator0
      ;[0 0 0] Single Orbit
      (CallFunction|Rotate DeltaSeconds)
      (bind _outpoint (CallFunction|GetRotationAroundPoint (Variables|Default|GetDistance) (Math|Vector|RotateVectorAroundAxis (Variables|Default|GetOrbit1) (Variables|Default|GetAngle) (Variables|Default|GetAxis)) (Transformation|GetActorLocation (Variables|Default|GetAtom1))))
      (if (Variables|Default|GetLerping)
        (bind (_complete _lerptime) (CallFunction|Lerp DeltaSeconds (Variables|Default|GetLerpSpeed)))
        (if _complete
          (Variables|Default|SetLerping false)
          (Transformation|SetActorLocation _outpoint false false :!label _label)
          (else
            (Transformation|SetActorLocation (Math|Interpolation|Ease "EaseInOut" _lerptime (Transformation|GetActorLocation) _outpoint 2.0) false false)))
        (elif (Variables|Default|GetThrown)
          (bind (_complete_2 _lerptime_2) (CallFunction|Lerp DeltaSeconds (Variables|Default|GetVelocity)))
          (if _complete_2
            (Transformation|SetActorLocation (Variables|Default|GetTargetPoint) false false)
            (Variables|Default|SetThrown false)
            (Variables|Default|SetLerping true)
            (else
              (Transformation|SetActorLocation (Math|Interpolation|Ease "EaseOut" _lerptime_2 (Variables|Default|GetThrowPoint) (Variables|Default|GetTargetPoint) 2.0) false false)))
          (else
            (goto _label)))))
    (:NewEnumerator6
      (switch Utilities|FlowControl|Switch|SwitchonOrbitStates (Variables|Default|GetOrbitState)
        (:NewEnumerator0
          (CallFunction|Rotate DeltaSeconds))))
    (:NewEnumerator3
      ;[0 0 0] Stopped
      (if (or (Utilities|Enum|NotEqual(Enum) (Variables|/Game/AtomicAlchemy/Blueprints/Atom.Atom_C|GetCurrentState _atom1) "NewEnumerator2") (Variables|Default|GetLerping))
        (bind _outpoint_2 (CallFunction|GetRotationAroundPoint (Variables|Default|GetDistance) (Math|Vector|RotateVectorAroundAxis "0, 0,1.000000" (Variables|Default|GetStopRot) (Math|Vector|Normalize (- (Math|Vector|MakeVector (.x _returnvalue_4) (.y _returnvalue_4) 0.0) (Math|Vector|MakeVector (.x _returnvalue_5) (.y _returnvalue_5) 0.0)))) (Transformation|GetActorLocation _atom1)))
        (if (Variables|Default|GetThrown)
          (bind (_complete_3 _lerptime_3) (CallFunction|Lerp DeltaSeconds (Variables|Default|GetVelocity)))
          (if _complete_3
            (Transformation|SetActorLocation (Variables|Default|GetTargetPoint) false false)
            (Variables|Default|SetThrown false)
            (Variables|Default|SetLerping true)
            (else
              (Transformation|SetActorLocation (Math|Interpolation|Ease "EaseOut" _lerptime_3 (Variables|Default|GetThrowPoint) (Variables|Default|GetTargetPoint) 2.0) false false)))
          (elif (Variables|Default|GetLerping)
            (bind (_complete_4 _lerptime_4) (CallFunction|Lerp DeltaSeconds (Variables|Default|GetLerpSpeed)))
            (if _complete_4
              (Variables|Default|SetThrown false)
              (Variables|Default|SetLerping false)
              (Transformation|SetActorLocation _outpoint_2 false false :!label _label_2)
              (else
                (Transformation|SetActorLocation (Math|Interpolation|Ease "EaseInOut" _lerptime_4 (Transformation|GetActorLocation) _outpoint_2 2.0) false false)))
            (else
              (goto _label_2))))))
    (:NewEnumerator4
      ;[0 0 0] Held
      (CallFunction|UpdateOverlapConnection)
      (if (not (== (Variables|Default|GetAtom1) 0))
        (CallFunction|UpdateSplineandMesh)
        (Variables|Default|SetThrowPoint (Variables|Default|GetTargetPoint))
        (Variables|Default|SetTargetPoint (Transformation|GetActorLocation))
        (Variables|Default|SetVelocity DeltaSeconds)))))

(event EventStopElectron
  (params (StopRot :type Float%20%28single-precision%29))
  ;[0 0 0] Stop and Start Electron
  (Variables|Default|SetStopRot StopRot)
  (Variables|Default|SetLerping true)
  (Variables|Default|SetStopped true)
  (if (Variables|Default|GetThrown)
    _
    (else
      (Variables|Default|SetLerpTime 0.0)))
  (Variables|Default|SetCurrentState "NewEnumerator3")
  (Components|Activation|Deactivate (Variables|Default|GetElectronTrail)))

(event EventStartElectron
  ;[0 0 0] Stop and Start Electron
  (Variables|Default|SetLerping true)
  (Variables|Default|SetStopped false)
  (if (Variables|Default|GetThrown)
    _
    (else
      (Variables|Default|SetLerpTime 0.0)))
  (CallFunction|UpdateConnectionState)
  (Components|Activation|Activate (Variables|Default|GetElectronTrail) false))

(event EventGrabElectron
  (params (GrabbedBy :type Scene%20Component%20Object%20Reference))
  ;[0 0 0] Grab and Release Electron
  (Components|Activation|Deactivate (Variables|Default|GetElectronTrail))
  (if (Utilities|Enum|Equal(Enum) (Variables|Default|GetCurrentState) "NewEnumerator5")
    _
    (else
      (Transformation|DetachFromActor "KeepWorld" "KeepWorld" "KeepWorld")))
  (Variables|Default|SetCurrentState "NewEnumerator4")
  (Transformation|AttachComponentToComponent GrabbedBy "None" "KeepWorld" "KeepWorld" "KeepWorld" true)
  (if (not (== (Variables|Default|GetAtom1) 0))
    (bind _returnvalue (Game|SpawnActorfromClass "/Game/AtomicAlchemy/Blueprints/ElectronConnection.ElectronConnection_C" (Math|Transform|MakeTransform "0, 0,0.000000") "Undefined" 0 0))
    (Variables|Default|SetSplineMesh _returnvalue)
    (Variables|Default|SetLerping false)
    (Variables|Default|SetThrown false)))

(fn ConstructionScript)

(fn GetRotationAroundPoint
  (params (Distance :type Float%20%28single-precision%29) (Rotation :type Vector) (Center :type Vector))
  (return (+ (* Rotation Distance) Center)))

(fn UpdateOverlapConnection
  (bind _array_element (Utilities|Array|ForEachLoopwithBreak (Collision|GetOverlappingActors (Variables|Default|GetStaticMesh) "/Game/AtomicAlchemy/Blueprints/Atom.Atom_C" :!class /Script/Engine.PrimitiveComponent))
    (:LoopBody
      (if (== 0 (Variables|Default|GetAtom1))
        (bind _asatom (Utilities|Casting|CastToAtom _array_element))
        (Variables|Default|SetAtom1 _asatom)
        (elif (not (== _array_element (Variables|Default|GetAtom1)))
          (if (== 0 (Variables|Default|GetAtom2))
            (bind _asatom_2 (Utilities|Casting|CastToAtom _array_element))
            (Variables|Default|SetAtom2 _asatom_2)
            (LocalVariables|SetAtom2Found true :!label _label)
            (elif (== _array_element (Variables|Default|GetAtom2))
              (goto _label)
              (else
                (bind _asatom_3 (Utilities|Casting|CastToAtom _array_element))
                (LocalVariables|SetAtom3 _asatom_3)))))))
    (:Completed
      (if (not (or (LocalVariables|GetAtom2Found) (!= 0 (LocalVariables|GetAtom3))))
        (Variables|Default|SetAtom2 (LocalVariables|GetAtom3))))))

(fn UpdateSplineandMesh
  (SplineMesh|SetStartandEnd (Variables|/Script/Engine.SplineMeshActor|GetSplineMeshComponent (Variables|Default|GetSplineMesh)) (Transformation|GetActorLocation (Variables|Default|GetAtom1)) "0, 0, 0" (Transformation|GetWorldLocation (Variables|Default|GetElectron)) "0, 0, 0" true :!class /Script/Engine.SplineMeshComponent) ; Set the tangents and position to build slightly bend the cylinder. All cylinders combined create a smooth arc.
)

(fn UpdateConnectionState
  (bind _atom1 (Variables|Default|GetAtom1))
  (if (Variables|Default|GetStopped)
    (Variables|Default|SetCurrentState "NewEnumerator3")
    (Class|NucleusInterface|ElectronReleased(Message) _atom1)
    (return)
    (else
      (if (== _atom1 0)
        (Variables|Default|SetCurrentState "NewEnumerator5")
        (elif (== 0 (Variables|Default|GetAtom2))
          (Variables|Default|SetCurrentState "NewEnumerator0")
          (else
            (Variables|Default|SetCurrentState "NewEnumerator6"))))
      (return))))

(fn CreateSingleOrbit
  (params (Orbit1 :type Vector))
  (bind _output_get (Variables|Default|SetOrbit1 Orbit1))
  (Variables|Default|SetRotSpeed (Math|Random|RandomFloatinRange 8e+01 1.2e+02))
  (Variables|Default|SetAngle (Math|Random|RandomFloatinRange 0.0 3.6e+02))
  (Variables|Default|SetAxis (Math|Vector|Normalize (Math|Vector|CrossProduct _output_get "0,1.000000, 0"))))

(fn Lerp
  (params (DeltaTime :type Float%20%28single-precision%29) (LerpSpeed :type Float%20%28single-precision%29))
  (if (>= (+ (Variables|Default|GetLerpTime) (* DeltaTime LerpSpeed)) 1.0)
    (bind _output_get (Variables|Default|SetLerpTime 0.0))
    (return true _output_get)
    (else
      (bind _output_get_2 (Variables|Default|SetLerpTime (+ (Variables|Default|GetLerpTime) (* DeltaTime LerpSpeed))))
      (return false _output_get_2))))

(fn Rotate
  (params (DeltaTime :type Float%20%28single-precision%29))
  (if (>= (+ (Variables|Default|GetAngle) (* DeltaTime (Variables|Default|GetRotSpeed))) 3.6e+02)
    (bind _output_get (Variables|Default|SetAngle (- (+ (Variables|Default|GetAngle) (* DeltaTime (Variables|Default|GetRotSpeed))) 3.6e+02)))
    (return _output_get)
    (else
      (bind _output_get_2 (Variables|Default|SetAngle (+ (Variables|Default|GetAngle) (* DeltaTime (Variables|Default|GetRotSpeed)))))
      (return _output_get_2))))

(fn SetThrowPoint
  (bind _throwpoint (Variables|Default|GetThrowPoint))
  (Variables|Default|SetTargetPoint (/ (- (Variables|Default|GetTargetPoint) _throwpoint) (Variables|Default|GetVelocity)))
  (bind _output_get (Variables|Default|SetVelocity (Math|Vector|VectorLength (Variables|Default|GetTargetPoint))))
  (Variables|Default|SetTargetPoint (+ _throwpoint (* (Variables|Default|GetTargetPoint) 1.0)))
  (Variables|Default|SetVelocity (Math|Float|Power (/ _output_get 1e+02) -0.1)))

(fn HalfRotate
  (params (DeltaTime :type Float%20%28single-precision%29) (StartingAngle :type Float%20%28single-precision%29))
  (if (>= (+ (Variables|Default|GetAngle) (* DeltaTime (Variables|Default|GetRotSpeed))) 3.6e+02)
    (bind _output_get (Variables|Default|SetAngle (- (+ (Variables|Default|GetAngle) (* DeltaTime (Variables|Default|GetRotSpeed))) 3.6e+02)))
    (return _output_get)
    (else
      (bind _output_get_2 (Variables|Default|SetAngle (+ (Variables|Default|GetAngle) (* DeltaTime (Variables|Default|GetRotSpeed)))))
      (return _output_get_2))))

(fn CreateDoubleOrbit
  (params (NewParam :type Vector)))

(fn AttachElectron
  (params (Electron :type Actor%20Object%20Reference))
  (return false "0, 0, 0"))

(fn ConnectElectron
  (params (Electron :type Actor%20Object%20Reference))
  (return false))

(fn DetachElectron
  (params (Electron :type Actor%20Object%20Reference))
  (return false))